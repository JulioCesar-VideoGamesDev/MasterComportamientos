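; AI controller from an exercise that makes its pawn chase the player with simple obstacle avoidance, without pathfinding.
; Tick, throttled by a short Delay, runs a debug-drawn visibility multi-trace from the pawn toward the player.
; A blocking hit steers MoveToLocation perpendicular to the right of that direction; otherwise it moves toward the player.
; Unconnected earlier stages remain: random wandering and forward-trace avoidance.
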(event EventBeginPlay)

(event EventTick
  (params (DeltaSeconds :type Float%20%28single-precision%29))
  (bind _returnvalue (Game|Player|GetPlayerPawn 0))
  (bind _returnvalue_2 (Pawn|GetControlledPawn))
  (bind _returnvalue_3 (Transformation|GetActorLocation _returnvalue))
  (bind _returnvalue_4 (Transformation|GetActorLocation _returnvalue_2))
  (bind _returnvalue_5 (Math|Vector|GetUnitDirection(Vector) _returnvalue_4 _returnvalue_3))
  (bind _returnvalue_6 (* _returnvalue_5 3e+02))
  (bind _returnvalue_7 (+ _returnvalue_4 _returnvalue_6))
  ;[0.15 0.15 0.15 0.5] Part3 ChasePlayer
  (Utilities|FlowControl|Delay 0.05)
  (bind _returnvalue_8 (Collision|MultiLineTraceByChannel _returnvalue_4 _returnvalue_7 "TraceTypeQuery1" false 0 "ForOneFrame"))
  (AI|Navigation|MovetoLocation (Math|Vector|SelectVector (+ (* (Math|Vector|GetRightVector (Math|Rotator|MakeRotfromX _returnvalue_5)) 3e+02) _returnvalue_4) _returnvalue_7 _returnvalue_8) -1.0 true false false true 0))

(fn ConstructionScript)