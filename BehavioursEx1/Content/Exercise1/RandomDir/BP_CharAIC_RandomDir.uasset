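; AI controller from an exercise that makes its pawn wander in random directions.
; Tick runs through a one-second Delay, then moves the pawn to a random horizontal offset from its location without pathfinding.
; Two unconnected variants remain in the graph: line-trace avoidance that sidesteps right when blocked ahead, and a player chase using the same sidestep with a multi-trace.
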(event EventBeginPlay)

(event EventTick
  (params (DeltaSeconds :type Float%20%28single-precision%29))
  ;[0.15 0.15 0.15 0.5] Part1 Random Direction
  (Utilities|FlowControl|Delay 1.0)
  (AI|Navigation|MovetoLocation (+ (Transformation|GetActorLocation (Pawn|GetControlledPawn)) (Math|Vector|MakeVector (Math|Random|RandomFloatinRange -3e+02 3e+02) (Math|Random|RandomFloatinRange -3e+02 3e+02) 0.0)) -1.0 true false false true 0))

(fn ConstructionScript)