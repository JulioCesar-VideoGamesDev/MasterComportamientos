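; AI controller for a ray-tracing exercise that steers its pawn around obstacles without pathfinding.
; Tick, throttled by a short Delay, fires a debug-drawn Visibility line trace ahead of the pawn.
; A hit moves the pawn to its right; otherwise it moves forward.
; Two disconnected exercise parts remain: random-direction wandering, and chasing the player with a multi-trace and the same right sidestep.
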(event EventBeginPlay)

(event EventTick
  (params (DeltaSeconds :type Float%20%28single-precision%29))
  (bind _returnvalue (Pawn|GetControlledPawn))
  (bind _returnvalue_2 (Transformation|GetActorLocation _returnvalue))
  (bind _returnvalue_3 (Transformation|GetActorForwardVector _returnvalue))
  (bind _returnvalue_4 (* _returnvalue_3 3e+02))
  (bind _returnvalue_5 (+ _returnvalue_2 _returnvalue_4))
  ;[0.15 0.15 0.15 0.5] Part2 RayTracing to avoid obstacles
  (Utilities|FlowControl|Delay 0.05)
  (bind _returnvalue_6 (Collision|LineTraceByChannel _returnvalue_2 _returnvalue_5 "TraceTypeQuery1" false 0 "ForOneFrame"))
  (AI|Navigation|MovetoLocation (Math|Vector|SelectVector (+ _returnvalue_2 (* (Transformation|GetActorRightVector _returnvalue) 3e+02)) _returnvalue_5 _returnvalue_6) -1.0 true false false true 0))

(fn ConstructionScript)