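; Behavior tree decorator that passes when the AI's controlled pawn is within an acceptable distance of its follow target.
; It casts the owner to BP_CharAIC, caches that reference, and reads the target actor from the TargetToFollow blackboard key.
; The check compares the straight-line distance between target and pawn against AcceptableDistance, and fails if the cast fails.
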(fn PerformConditionCheck
  (params (OwnerActor :type Actor%20Object%20Reference))
  (bind _asbp_char_aic (Utilities|Casting|CastToBP_CharAIC OwnerActor)
    (:then
      (bind _output_get (Variables|Default|SetAICtrlRef _asbp_char_aic))
      (return (<= (Math|Vector|VectorLength (- (Transformation|GetActorLocation (AI|BehaviorTree|GetBlackboardValueasActor (Variables|Default|GetTargetToFollow))) (Transformation|GetActorLocation (Pawn|GetControlledPawn _output_get)))) (Variables|Default|GetAcceptableDistance))))
    (:CastFailed
      (return false))))