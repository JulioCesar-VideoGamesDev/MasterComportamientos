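; Behavior Tree service that cycles a BP_CharAI pawn through its waypoint route.
; While active, it binds to the BP_CharAIC controller's move-completed event and unbinds on deactivation.
; On a successful or invalid result, it advances RouteIdx with wraparound and writes that waypoint's position to the WaypointLocation blackboard key.
; Invalid results are accepted because the author relies on one to start the first move.
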(event Custom|ReceiveMoveCompleted_Event
  (params (RequestID :type AI%20Request%20ID%20Structure) (Result :type EPathFollowingResult%20Enum :default "Success"))
  (bind _routeidx (Variables|Default|GetRouteIdx))
  (bind _returnvalue (Class|BTFunctionLibrary|GetBlackboardValueasInt _routeidx))
  (switch Utilities|FlowControl|Switch|SwitchonEPathFollowingResult Result ; Im conecting the Invalid too, bc the first time this gets called will always be invalid\nbc if I don't call this to set a position then the AI wont move
    (:Success
      _)
    (:Invalid
      _))
  (bind _asbp_char_ai (Utilities|Casting|CastToBP_CharAI (Pawn|GetControlledPawn (Variables|Default|GetAICtrRef))))
  (Class|BTFunctionLibrary|SetBlackboardValueasInt (Variables|Default|GetRouteIdx) (Math|Integer|%(Integer) (+ _returnvalue 1) (Utilities|Array|Length (Variables|/Game/Exercise3/BP_CharAI.BP_CharAI_C|GetWayPoints _asbp_char_ai))))
  (AI|BehaviorTree|SetBlackboardValueasVector (Variables|Default|GetWaypointLocation) (Transformation|GetActorLocation (Utilities|Array|Get(acopy) (Variables|/Game/Exercise3/BP_CharAI.BP_CharAI_C|GetWayPoints _asbp_char_ai) _returnvalue))))

(event EventReceiveActivation
  (params (OwnerActor :type Actor%20Object%20Reference))
  (bind _asbp_char_aic (Utilities|Casting|CastToBP_CharAIC OwnerActor))
  (EventDispatchers|BindEventtoReceiveMoveCompleted _asbp_char_aic (delegate Custom|ReceiveMoveCompleted_Event))
  (Variables|Default|SetAICtrRef _asbp_char_aic))

(event EventReceiveDeactivation
  (params (OwnerActor :type Actor%20Object%20Reference))
  (bind _asbp_char_aic (Utilities|Casting|CastToBP_CharAIC OwnerActor))
  (EventDispatchers|UnbindEventfromReceiveMoveCompleted _asbp_char_aic (delegate Custom|ReceiveMoveCompleted_Event))
  (Variables|Default|SetAICtrRef 0))