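; Behavior tree task that sends an AI-controlled pawn toward the actor stored in the TargetToFollow blackboard key.
; It casts the owner to BP_CharAIC on first use, caches that controller, and issues AIMoveTo on its pawn.
; It finishes successfully from the immediate output without waiting for arrival.
; A missing target or failed cast leaves the task without a FinishExecute call.
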(event EventReceiveExecute
  (params (OwnerActor :type Actor%20Object%20Reference))
  (if (!= (AI|BehaviorTree|GetBlackboardValueasActor (Variables|Default|GetTargetToFollow)) 0)
    (if (!= (Variables|Default|GetAICtrlRef) 0)
      _
      (else
        (bind _asbp_char_aic (Utilities|Casting|CastToBP_CharAIC OwnerActor))
        (Variables|Default|SetAICtrlRef _asbp_char_aic)))
    (AI|AIMoveTo (Pawn|GetControlledPawn (Variables|Default|GetAICtrlRef)) "0, 0, 0" (AI|BehaviorTree|GetBlackboardValueasActor (Variables|Default|GetTargetToFollow)) 5.0 false
      (:then
        (AI|BehaviorTree|FinishExecute true)))))