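; AI controller that keeps an AI_Character_Ej2 wandering between the TargetPoint_Ej2 actors that allow it.
; On BeginPlay and one second after each move completes, it appends eligible points to Routes without clearing the array.
; It reshuffles until the first point is unlocked, then locks it, releases the previous one and moves there.
; Locking reserves destinations, but the retry loop has no exit if every candidate is locked.
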(event Custom|ReceiveMoveCompleted_Event
  (params (RequestID :type AI%20Request%20ID%20Structure) (Result :type EPathFollowingResult%20Enum :default "Success"))
  (bind _routes (Variables|Default|GetRoutes))
  (bind _output (Utilities|Array|Get(acopy) _routes))
  (Utilities|FlowControl|Delay 1.0)
  (bind _outactors (Actor|GetAllActorsOfClass "/Game/BluePrints/Ejercicio2/TargetPoint_Ej2.TargetPoint_Ej2_C"))
  (bind _asai_character_ej_2 (Utilities|Casting|CastToAI_Character_Ej2 (Pawn|GetControlledPawn)))
  (for _array_element _outactors
    (if (!= (Utilities|Array|FindItem (Variables|/Game/BluePrints/Ejercicio2/TargetPoint_Ej2.TargetPoint_Ej2_C|GetAllowedCharacters _array_element) _asai_character_ej_2) -1)
      (Utilities|Array|Add (Variables|Default|GetRoutes) _array_element)))
  (if (> (Utilities|Array|Length _routes) 0)
    (Utilities|Array|Shuffle _routes :!label _label)
    (if (not (Variables|/Game/BluePrints/Ejercicio2/TargetPoint_Ej2.TargetPoint_Ej2_C|GetLocked _output))
      (Utilities|IsValid (Variables|Default|GetOldRoute)
        (:Is%20Valid
          (Variables|/Game/BluePrints/Ejercicio2/TargetPoint_Ej2.TargetPoint_Ej2_C|SetLocked (Variables|Default|GetOldRoute) false))
        (:Is%20Not%20Valid
          _))
      (Variables|/Game/BluePrints/Ejercicio2/TargetPoint_Ej2.TargetPoint_Ej2_C|SetLocked _output true)
      (Variables|Default|SetOldRoute _output)
      (AI|Navigation|MovetoLocation (Transformation|GetActorLocation _output) 1e+01 true true true true 0)
      (else
        (Development|PrintText "a")
        (goto _label)))))

(event EventBeginPlay
  (bind _routes (Variables|Default|GetRoutes))
  (bind _output (Utilities|Array|Get(acopy) _routes))
  (EventDispatchers|BindEventtoReceiveMoveCompleted (delegate Custom|ReceiveMoveCompleted_Event))
  (bind _outactors (Actor|GetAllActorsOfClass "/Game/BluePrints/Ejercicio2/TargetPoint_Ej2.TargetPoint_Ej2_C"))
  (bind _asai_character_ej_2 (Utilities|Casting|CastToAI_Character_Ej2 (Pawn|GetControlledPawn)))
  (for _array_element _outactors
    (if (!= (Utilities|Array|FindItem (Variables|/Game/BluePrints/Ejercicio2/TargetPoint_Ej2.TargetPoint_Ej2_C|GetAllowedCharacters _array_element) _asai_character_ej_2) -1)
      (Utilities|Array|Add (Variables|Default|GetRoutes) _array_element)))
  (if (> (Utilities|Array|Length _routes) 0)
    (Utilities|Array|Shuffle _routes :!label _label)
    (if (not (Variables|/Game/BluePrints/Ejercicio2/TargetPoint_Ej2.TargetPoint_Ej2_C|GetLocked _output))
      (Utilities|IsValid (Variables|Default|GetOldRoute)
        (:Is%20Valid
          (Variables|/Game/BluePrints/Ejercicio2/TargetPoint_Ej2.TargetPoint_Ej2_C|SetLocked (Variables|Default|GetOldRoute) false))
        (:Is%20Not%20Valid
          _))
      (Variables|/Game/BluePrints/Ejercicio2/TargetPoint_Ej2.TargetPoint_Ej2_C|SetLocked _output true)
      (Variables|Default|SetOldRoute _output)
      (AI|Navigation|MovetoLocation (Transformation|GetActorLocation _output) 1e+01 true true true true 0)
      (else
        (Development|PrintText "a")
        (goto _label)))))

(event EventTick
  (params (DeltaSeconds :type Float%20%28single-precision%29)))

(fn ConstructionScript)