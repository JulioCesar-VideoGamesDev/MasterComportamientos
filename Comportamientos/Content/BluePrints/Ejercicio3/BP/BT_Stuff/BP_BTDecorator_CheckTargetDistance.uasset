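; Behavior tree decorator that passes when the AI's controlled pawn is within an acceptable distance of its follow target.
; It casts the owner to BP_CharAIC_Ej3, stores that controller, and reads the target actor from the TargetToFollow blackboard key.
; The straight-line distance between the two actor locations is compared to AcceptableDistance, and a failed cast returns false.
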(fn PerformConditionCheck
  (params (OwnerActor :type Actor%20Object%20Reference))
  (bind _asaic_character_ej_3 (Utilities|Casting|CastToBP_CharAIC_Ej3 OwnerActor)
    (:then
      (bind _output_get (Variables|Default|SetAICtrlRef _asaic_character_ej_3))
      (return (<= (Math|Vector|VectorLength (- (Transformation|GetActorLocation (AI|BehaviorTree|GetBlackboardValueasActor (Variables|Default|GetTargetToFollow))) (Transformation|GetActorLocation (Pawn|GetControlledPawn _output_get)))) (Variables|Default|GetAcceptableDistance))))
    (:CastFailed
      (return false))))