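; Behavior tree service that finds a visible target near an AI pawn and writes it to the blackboard.
; Each tick, using a cached BP_CharAIC_Ej3 controller, it sphere-traces around the pawn for the desired object types, ignoring all BP_CharAI_Ej3 actors.
; A Camera-channel line trace checks each hit's visibility; the first visible one sets TargetToFollow and TargetLocation.
; Blocked hits clear only TargetToFollow, so TargetLocation keeps the last seen position.
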(event EventReceiveTickAI
  (params (OwnerController :type AI%20Controller%20Object%20Reference) (ControlledPawn :type Pawn%20Object%20Reference) (DeltaSeconds :type Float%20%28single-precision%29))
  (bind _targettofollow (Variables|Default|GetTargetToFollow))
  (if (!= (Variables|Default|GetAICtrlRef) 0)
    _
    (else
      (bind _asaic_character_ej_3 (Utilities|Casting|CastToBP_CharAIC_Ej3 OwnerController))
      (Variables|Default|SetAICtrlRef _asaic_character_ej_3)))
  (Variables|Default|SetMyLocation (Transformation|GetActorLocation (Pawn|GetControlledPawn (Variables|Default|GetAICtrlRef))))
  (bind _outactors (Actor|GetAllActorsOfClass "/Game/BluePrints/Ejercicio3/BP/BP_CharAI_Ej3.BP_CharAI_Ej3_C"))
  (bind _outhits (Collision|MultiSphereTraceForObjects (Variables|Default|GetMyLocation) (+ (Variables|Default|GetMyLocation) "0.000000,0.000000,15.000000") 1.5e+03 (Variables|Default|GetDesiredObjectTypes) false _outactors "ForOneFrame" :!pinned true)) ; We detect all pawns that suround us but ignoring\nthe AIs
  (bind _array_element (Utilities|Array|ForEachLoopwithBreak _outhits :!label _label)
    (:LoopBody
      (bind _outhit (Collision|LineTraceByChannel (Variables|Default|GetMyLocation) (Transformation|GetActorLocation (.HitActor (Collision|BreakHitResult _array_element))) "TraceTypeQuery2" false _outactors "ForOneFrame" :!pinned true)) ; So the way that we check if the pawn that we are\nhitting is the player, is by the TraceChannel?\nAlso obviously this is used to check if we can see\nthe player or not.
      (if (== (.HitActor (Collision|BreakHitResult _outhit)) (.HitActor (Collision|BreakHitResult _array_element)))
        (Class|BTFunctionLibrary|SetBlackboardValueasObject _targettofollow (.HitActor (Collision|BreakHitResult _outhit)))
        (AI|BehaviorTree|SetBlackboardValueasVector (Variables|Default|GetTargetLocation) (Transformation|GetActorLocation (.HitActor (Collision|BreakHitResult _outhit))))
        (goto _label Break)
        (else
          (Class|BTFunctionLibrary|SetBlackboardValueasObject _targettofollow))))))