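; Behavior tree task that sends the AI-controlled pawn toward the actor stored in the TargetToFollow blackboard key.
; On execute it casts the owner to BP_CharAIC_Ej3, caches that controller, and calls AIMoveTo on its pawn.
; The task reports success as soon as the move is issued, without waiting for arrival or failure.
; A failed cast leaves the task unfinished.
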(event EventReceiveExecute
  (params (OwnerActor :type Actor%20Object%20Reference))
  (if (!= (Variables|Default|GetAICtrlRef) 0)
    _
    (else
      (bind _asaic_character_ej_3 (Utilities|Casting|CastToBP_CharAIC_Ej3 OwnerActor))
      (Variables|Default|SetAICtrlRef _asaic_character_ej_3)))
  (AI|AIMoveTo (Pawn|GetControlledPawn (Variables|Default|GetAICtrlRef)) "0, 0, 0" (AI|BehaviorTree|GetBlackboardValueasActor (Variables|Default|GetTargetToFollow)) 5.0 false
    (:then
      (AI|BehaviorTree|FinishExecute true))))